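; BP_Collisions is a spline actor that builds collision geometry along an editable path.
; Its Construction Script adds one spline mesh per segment, using world-space locations and tangents with manual attachment so each piece follows the curve.
; Each piece gets the assigned mesh, a fixed cross-section scale, query-and-physics collision and a custom object channel.
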(fn ConstructionScript
  (bind _spline (Variables|Default|GetSpline))
  ;[0.15 0.15 0.15 0.5] Make Spline Have a Static Mesh
  (for _index (range 0 (- (Spline|GetNumberOfSplinePoints (Variables|Default|GetSpline)) 2))
    (bind _returnvalue (AddComponent|AddSplineMeshComponent true))
    (bind _output_get (Variables|Default|SetSplineMesh _returnvalue))
    (Components|StaticMesh|SetStaticMesh _output_get (Variables|Default|GetNewMesh))
    (SplineMesh|SetStartandEnd (Variables|Default|GetSplineMesh) (.Location (Spline|GetLocationandTangentatSplinePoint _spline _index "World")) (.Tangent (Spline|GetLocationandTangentatSplinePoint _spline _index "World")) (.Location (Spline|GetLocationandTangentatSplinePoint _spline (+ _index 1) "World")) (.Tangent (Spline|GetLocationandTangentatSplinePoint _spline (+ _index 1) "World")) true :!class /Script/Engine.SplineMeshComponent)
    ;[0.15 0.15 0.15 0.5] Change Static Mesh Scale
    (SplineMesh|SetStartScale (Variables|Default|GetSplineMesh) "(X=0.500000,Y=0.200000)" true :!class /Script/Engine.SplineMeshComponent)
    (SplineMesh|SetEndScale (Variables|Default|GetSplineMesh) "(X=0.500000,Y=0.200000)" true :!class /Script/Engine.SplineMeshComponent)
    ;[0.15 0.15 0.15 0.5] Collision Configuration
    (Collision|SetCollisionEnabled (Variables|Default|GetSplineMesh) "QueryAndPhysics")
    (Collision|SetCollisionObjectType (Variables|Default|GetSplineMesh) "ECC_GameTraceChannel1")))