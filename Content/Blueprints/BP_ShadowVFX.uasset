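; Shadow VFX actor that shows a brief effect on the player whenever the game switches between 2D and 3D perspective.
; On BeginPlay it caches the player's 2D and 3D cameras through message calls.
; PerspectiveChange reveals the VFX for 1.5 seconds.
; While active, Tick moves the actor to the player and billboards the VFX toward the current mode's camera with a pitch offset.
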(event Custom|PerspectiveChange
  (params (is2D :type Boolean))
  (Variables|Default|Setis2D is2D)
  (Variables|Default|SetIsActive true)
  (Rendering|SetVisibility (Variables|Default|GetVFX) true false)
  (Utilities|FlowControl|Delay 1.5)
  (Variables|Default|SetIsActive false)
  (Rendering|SetVisibility (Variables|Default|GetVFX) false false))

(event Custom|FollowPlayer
  (Transformation|SetWorldLocation (Variables|Default|GetDefaultSceneRoot) (Transformation|GetActorLocation (Game|GetPlayerCharacter 0)) false true))

(event Custom|LookAtCamera
  (params (Camera :type Camera%20Component%20Object%20Reference))
  (bind _returnvalue (Transformation|GetWorldLocation Camera))
  (bind _vfx (Variables|Default|GetVFX))
  (bind _returnvalue_2 (Transformation|GetWorldLocation _vfx))
  (bind _returnvalue_3 (Math|Rotator|FindLookatRotation _returnvalue_2 _returnvalue))
  (bind (_roll _pitch _yaw) (Math|Rotator|BreakRotator _returnvalue_3))
  (Transformation|SetWorldRotation (Variables|Default|GetVFX) (Math|Rotator|MakeRotator _roll (+ _pitch -9e+01) _yaw) false true))

(event EventTick
  (params (DeltaSeconds :type Float%20%28single-precision%29))
  (if (Variables|Default|GetIsActive)
    (CallFunction|FollowPlayer)
    (if (Variables|Default|Getis2D)
      (CallFunction|LookatCamera (Variables|Default|Get2DCamera))
      (else
        (CallFunction|LookatCamera (Variables|Default|Get3DCamera))))))

(event EventBeginPlay
  (bind _returnvalue (Game|GetPlayerCharacter 0))
  (bind _2dcamera (Class|BPIInteraction|GetCamera2D(Message) _returnvalue))
  (Variables|Default|Set2DCamera _2dcamera)
  (bind _3dcamera (Class|BPIInteraction|GetCamera3D(Message) _returnvalue))
  (Variables|Default|Set3DCamera _3dcamera))

(fn ConstructionScript)